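; BP_PlayerPawn is the player pawn, carrying a spring-arm camera rig that is configured before play.
; The Construction Script sets the arm's pitch from CameraPitch, keeping its roll and yaw.
; When FocusActor is valid, it also moves the arm to that actor's location and applies the configured arm length.
; The event graph holds only disabled placeholders, so the pawn's graphs have no runtime logic.
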(event EventBeginPlay)

(event Collision|EventActorBeginOverlap
  (params (OtherActor :type Actor%20Object%20Reference)))

(event EventTick
  (params (DeltaSeconds :type Float%20%28single-precision%29)))

(fn ConstructionScript
  (bind _springarm (Variables|Default|GetSpringArm))
  (bind _relativerotation (Variables|/Script/Engine.SceneComponent|GetRelativeRotation _springarm))
  ;[1 1 1] Настройки камеры (До запуска проекта)
  (Transformation|SetRelativeRotation _springarm (Math|Rotator|MakeRotator (.roll _relativerotation) (Variables|Additionals|GetCameraPitch) (.yaw _relativerotation)) false false)
  (Utilities|IsValid (Variables|Additionals|GetFocusActor)
    (:Is%20Valid
      (Transformation|SetWorldLocation (Variables|Default|GetSpringArm) (Transformation|GetActorLocation (Variables|Additionals|GetFocusActor)) false false)
      (Variables|/Script/Engine.SpringArmComponent|SetTargetArmLength (Variables|Default|GetSpringArm) (Variables|Additionals|GetTargetArmLenght)))))