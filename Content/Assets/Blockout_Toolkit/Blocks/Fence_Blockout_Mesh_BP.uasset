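; Blockout fence Blueprint that builds a procedural fence along an editable spline in its construction script.
; An unrotated box post stands at each spline point, with evenly stacked beams running straight between neighboring points, ignoring curvature, and optionally closing the loop.
; All boxes accumulate into one procedural mesh section with collision, using the material instance from the parent toolkit setup.
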(fn ConstructionScript
  (|CallParentFunction)
  (CallFunction|Create&GetMaterialInstance)
  (CallFunction|GenerateFence))

(fn GenerateFence
  (bind _spline (Variables|Default|GetSpline))
  (bind _beams_size (Variables|Settings|GetBeams%20Size))
  (bind _returnvalue (Spline|GetNumberOfSplinePoints _spline))
  (bind _returnvalue_2 (/ _beams_size 2))
  (bind (_x _y _z) (Math|Vector|BreakVector _returnvalue_2))
  (Spline|SetClosedLoop (Variables|Default|GetSpline) (Variables|Settings|GetClosed%20Loop?) true)
  (if (> _returnvalue 0)
    (Utilities|FlowControl|Sequence
      (:then_0
        (for _index (range 0 (- _returnvalue 1))
          (LocalVariables|SetLocalPointIndex _index)
          (CallFunction|CreateBoxMeshwithRotation (+ (.Location (Math|Transform|BreakTransform (Spline|GetTransformatSplinePoint (Variables|Default|GetSpline) _index "Local" false))) (Math|Vector|MakeVector 0.0 0.0 (/ (.Z (Class|KismetMathLibrary|BreakVector3f (Variables|Settings|GetPosts%20Size))) 2.0))) "0, 0, 0" (/ (Variables|Settings|GetPosts%20Size) 2.0) (LocalVariables|GetLocalVertices) (LocalVariables|GetLocalTriangles) (LocalVariables|GetLocalNormals) (LocalVariables|GetLocalUVs))
          (if (or (< (LocalVariables|GetLocalPointIndex) (- (Spline|GetNumberOfSplinePoints (Variables|Default|GetSpline)) 1)) (Variables|Settings|GetClosed%20Loop?))
            (LocalVariables|SetLocalBeamOffset (/ (.Z (Math|Vector|BreakVector (/ (Variables|Settings|GetPosts%20Size) 2))) (Variables|Settings|GetBeams%20Amount)))
            (for _index_2 (range 1 (Variables|Settings|GetBeams%20Amount))
              (CallFunction|CreateBoxMeshwithRotation (+ (.Location (Math|Transform|BreakTransform (Spline|GetTransformatSplinePoint (Variables|Default|GetSpline) (LocalVariables|GetLocalPointIndex) "Local" false))) (* (- (.Location (Math|Transform|BreakTransform (Spline|GetTransformatSplinePoint (Variables|Default|GetSpline) (+ (LocalVariables|GetLocalPointIndex) 1) "Local" false))) (.Location (Math|Transform|BreakTransform (Spline|GetTransformatSplinePoint (Variables|Default|GetSpline) (LocalVariables|GetLocalPointIndex) "Local" false)))) 0.5) (Math|Vector|MakeVector 0.0 0.0 (LocalVariables|GetLocalBeamOffset))) (Math|Conversions|RotationFromXVector (- (.Location (Math|Transform|BreakTransform (Spline|GetTransformatSplinePoint (Variables|Default|GetSpline) (+ (LocalVariables|GetLocalPointIndex) 1) "Local" false))) (.Location (Math|Transform|BreakTransform (Spline|GetTransformatSplinePoint (Variables|Default|GetSpline) (LocalVariables|GetLocalPointIndex) "Local" false))))) (Math|Vector|MakeVector (* (Math|Vector|VectorLength (- (.Location (Math|Transform|BreakTransform (Spline|GetTransformatSplinePoint (Variables|Default|GetSpline) (+ (LocalVariables|GetLocalPointIndex) 1) "Local" false))) (.Location (Math|Transform|BreakTransform (Spline|GetTransformatSplinePoint (Variables|Default|GetSpline) (LocalVariables|GetLocalPointIndex) "Local" false))))) 0.5) _y _z) (LocalVariables|GetLocalVertices) (LocalVariables|GetLocalTriangles) (LocalVariables|GetLocalNormals) (LocalVariables|GetLocalUVs))
              (LocalVariables|SetLocalBeamOffset (+ (LocalVariables|GetLocalBeamOffset) (/ (.Z (Math|Vector|BreakVector (Variables|Settings|GetPosts%20Size))) (Variables|Settings|GetBeams%20Amount))))))))
      (:then_1
        (Class|ProceduralMeshComponent|CreateMeshSectionLinearColor (Variables|Default|GetProcMesh) 0 (LocalVariables|GetLocalVertices) (LocalVariables|GetLocalTriangles) (LocalVariables|GetLocalNormals) (LocalVariables|GetLocalUVs) 0 0 0 0 0 true false)
        (Rendering|Material|SetMaterial (Variables|Default|GetProcMesh) 0 (Variables|Default|GetMaterial%20Instance))))))